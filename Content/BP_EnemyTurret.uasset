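; BP_EnemyTurret is an enemy turret that turns its Sphere component to face the player.
; Every Tick it sets the Sphere's world rotation from a look-at rotation between the actor and player character 0, with pitch negated.
; An unfinished, unconnected shooting chain would spawn a BP_Arrow after a delay, using the actor's rotation at a fixed height, so the turret never fires.
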(event EventTick
  (params (DeltaSeconds :type Float%20%28single-precision%29))
  (bind _returnvalue (Game|GetPlayerCharacter 0))
  (bind _returnvalue_2 (Transformation|GetActorLocation))
  (bind _returnvalue_3 (Transformation|GetActorLocation _returnvalue))
  (bind _returnvalue_4 (Math|Rotator|FindLookatRotation _returnvalue_2 _returnvalue_3))
  ;[1 1 1] Makes the enemy turn towards the player
  (Transformation|SetWorldRotation (Variables|Default|GetSphere) (Math|Rotator|MakeRotator (.roll _returnvalue_4) (* (.pitch _returnvalue_4) -1.0) (.yaw _returnvalue_4)) false false))

(fn ConstructionScript)