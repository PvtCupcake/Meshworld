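; BP_PlayerChar1 is a player Blueprint that turns to face the mouse cursor and performs a sword melee attack.
; Each tick it deprojects the cursor, line traces against WorldStatic objects and sets the actor's yaw toward the hit location.
; Pressing MeleeAttack enables SwordCollision and plays a timeline that swings SwordPivot in yaw.
; Releasing disables the collision and reverses the swing, so the sword collides only while the input is held.
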(event EventBeginPlay
  (Collision|SetCollisionEnabled (Variables|Default|GetSwordCollision) "NoCollision"))

(event Collision|EventActorBeginOverlap
  (params (OtherActor :type Actor%20Object%20Reference)))

(event EventTick
  (params (DeltaSeconds :type Float%20%28single-precision%29))
  (bind _returnvalue (Game|GetPlayerController 0))
  (bind (_worldlocation _worlddirection) (Game|Player|ConvertMouseLocationToWorldSpace _returnvalue))
  ;[1 1 1] Rotate after Cursor
  (bind _outhit (Collision|LineTraceForObjects _worldlocation (+ _worldlocation (* _worlddirection 2000)) (Utilities|Array|MakeArray "ObjectTypeQuery1") false 0 "None"))
  (Transformation|SetActorRotation (Math|Rotator|MakeRotator 0.0 0.0 (.yaw (Math|Rotator|FindLookatRotation (Transformation|GetActorLocation) (.Location (Collision|BreakHitResult _outhit)))))))

(event Input|ActionEvents|InputActionMeleeAttack
  (params (Key :type Key%20Structure))
  (bind _swordcollision (Variables|Default|GetSwordCollision))
  ;[1 1 1] MeleeAttack
  (:Pressed
    (Collision|SetCollisionEnabled _swordcollision "QueryAndPhysics")
    (bind _swordswing (Timeline|SwordAttack Play)
      (:Update
        (Transformation|SetRelativeRotation (Variables|Default|GetSwordPivot) (Math|Rotator|MakeRotator 0.0 0.0 _swordswing) false false))))
  (:Released
    (Collision|SetCollisionEnabled _swordcollision "NoCollision")
    (Timeline|SwordAttack Reverse)))

(fn ConstructionScript)